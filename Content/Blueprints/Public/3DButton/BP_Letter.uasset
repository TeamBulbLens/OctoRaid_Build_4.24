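; BP_Letter is a one-shot 3D text button that spells its Text with centred BP_Char mesh actors for letters, digits and periods, sizing its collision box to fit.
; External Highlight calls tint the letters, and Tick clears the tint unless it is refreshed each frame.
; A motion controller overlap on the authority triggers ClickServer and ClickMulticast, which recolour the letters, release them into physics, play a sound, then fire OnButtonClick after a delay.
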(event OnComponentBeginOverlap(Box)
  (params (OverlappedComponent :type Primitive%20Component%20Object%20Reference) (OtherActor :type Actor%20Object%20Reference) (OtherComp :type Primitive%20Component%20Object%20Reference) (OtherBodyIndex :type Integer) (bFromSweep :type Boolean) (SweepResult :type Hit%20Result%20Structure%20%28by%20ref%29))
  ;[1 1 1] OnOverlaped
  (Networking|SwitchHasAuthority
    (:Authority
      (if (Variables|Default|GetClickable)
        (Utilities|Casting|CastToBP_MotionControllerMain OtherActor)
        (Variables|Default|SetClickable false)
        (CallFunction|HighlightBack)
        (CallFunction|ClickServer)))))

(event Custom|SetText
  (bind _returnvalue (Transformation|GetActorScale3D))
  (bind _box (Variables|Default|GetBox))
  (bind _boxextent (Variables|/Script/Engine.BoxComponent|GetBoxExtent _box))
  ;[1 1 1] 알파벳 글자 생성 + 배치
  (Variables|Default|SetSize (Utilities|Array|Length (Utilities|String|GetCharacterArrayfromString (Variables|Default|GetText))))
  (for (_array_element _array_index) (Utilities|String|GetCharacterArrayfromString (Class|KismetStringLibrary|ToUpper (Variables|Default|GetText)))
    (bind _outputpin (CallFunction|FindLetterMesh _array_element))
    (Transformation|SetActorRelativeLocation _outputpin (Math|Vector|MakeVector 0.0 (/ (+ (* (* (Variables|Default|GetSize) (Variables|Default|GetSpace)) 0.5) (* _array_index (* (Variables|Default|GetSpace) -1.0)) (* (Variables|Default|GetSpace) 0.5 -1.0)) (.y (.scale (Transformation|GetActorTransform)))) 0.0)))
  ;;[1 1 1] 전체 콜리전 박스 크기 설정
  (Components|Box|SetBoxExtent (Variables|Default|GetBox) (Math|Vector|MakeVector (* (.x _returnvalue) (.x _boxextent)) (* (Variables|Default|GetSize) (* (.y _returnvalue) (.y _boxextent))) (* (.z _returnvalue) (.z _boxextent))) false))

(event Custom|OnButtonClick
  ;[1 1 1] OnOverlaped
)

(event Custom|ClickMulticast
  ;[1 1 1] OnOverlaped
  (for _array_element (Actor|GetAttachedActors true)
    (bind _asbp_char (Utilities|Casting|CastToBP_Char _array_element))
    (Rendering|Material|SetScalarParameterValueonMaterials (Variables|/Game/Blueprints/Public/3DButton/BP_Char.BP_Char_C|GetStaticMesh _asbp_char) "Color" (Utilities|Select :Index (Variables|Default|GetSelectedColor) :NewEnumerator0 0.01 :NewEnumerator1 0.1 :NewEnumerator2 0.2 :NewEnumerator3 0.3 :NewEnumerator4 0.4 :NewEnumerator10 0.5 :NewEnumerator5 0.6 :NewEnumerator6 0.7 :NewEnumerator9 1.0))
    (Collision|SetCollisionEnabled (Variables|/Game/Blueprints/Public/3DButton/BP_Char.BP_Char_C|GetStaticMesh _asbp_char) "QueryAndPhysics")
    (Physics|SetSimulatePhysics (Variables|/Game/Blueprints/Public/3DButton/BP_Char.BP_Char_C|GetStaticMesh _asbp_char) true))
  (Audio|SpawnSoundatLocation "/Game/Ultimate_SFX_Bundle/Casual_Bundle/UI_Item_Sounds/Cues/8_Bit_click_sounds/8_Bit_click_sounds_7_Cue.8_Bit_click_sounds_7_Cue" (Transformation|GetActorLocation) "0, 0, 0" 1.0 1.0 0.0 0 0)
  (Utilities|FlowControl|Delay 1.0)
  (CallFunction|OnButtonClick))

(event Custom|ClickServer
  ;[1 1 1] OnOverlaped
  (CallFunction|ClickMulticast))

(event EventHighlight
  ;[1 1 1] Highlight
  (if (Variables|Default|GetClickable)
    (for _array_element (Actor|GetAttachedActors true)
      (bind _asbp_char (Utilities|Casting|CastToBP_Char _array_element))
      (Rendering|Material|SetVectorParameterValueonMaterials (Variables|/Game/Blueprints/Public/3DButton/BP_Char.BP_Char_C|GetStaticMesh _asbp_char) "HighlightColor" "0.100000,0.100000,0.100000")
      (Variables|Default|SetIsHightlighted true))))

(event EventHighlightBack
  ;[1 1 1] Highlight
  (if (Variables|Default|GetClickable)
    (for _array_element (Actor|GetAttachedActors true)
      (bind _asbp_char (Utilities|Casting|CastToBP_Char _array_element))
      (Rendering|Material|SetVectorParameterValueonMaterials (Variables|/Game/Blueprints/Public/3DButton/BP_Char.BP_Char_C|GetStaticMesh _asbp_char) "HighlightColor" "0, 0, 0"))))

(event EventTick
  (params (DeltaSeconds :type Float%20%28single-precision%29))
  ;[1 1 1] highlight 상태 업데이트
  (if (Variables|Default|GetClickable)
    (if (Variables|Default|GetIsHightlighted)
      (Variables|Default|SetIsHightlighted false)
      (else
        (CallFunction|HighlightBack)))))

(event EventBeginPlay
  ;[1 1 1] Init
  (CallFunction|SetText)
  (Variables|Default|SetSpace (* (.y (.scale (Transformation|GetActorTransform))) (Variables|Default|GetLetterWidth))))

(fn ConstructionScript)

(fn FindLetterMesh
  (params (SourceString :type String))
  (Variables|Default|SetcurLetter (Utilities|String|GetCharacterasNumber SourceString))
  (if (== (Variables|Default|GetcurLetter) 46)
    ;[1 1 1] 마침표일 경우
    (Variables|Default|SetcurLetter 36)
    (elif (> (Variables|Default|GetcurLetter) 64)
      ;[1 1 1] 알파벳일 경우
      (Variables|Default|SetcurLetter (- (Variables|Default|GetcurLetter) 65))
      (else
        ;[1 1 1] 숫자일 경우
        (Variables|Default|SetcurLetter (+ (- (Variables|Default|GetcurLetter) 48) 26)))))
  (if (< (Variables|Default|GetcurLetter) 37)
    (bind _returnvalue (Game|SpawnActorfromClass "/Game/Blueprints/Public/3DButton/BP_Char.BP_Char_C" (Transformation|GetActorTransform) "AlwaysSpawn" 0 0))
    (Transformation|AttachActorToActor _returnvalue self "None" "SnapToTarget" "SnapToTarget" "KeepRelative" false)
    (Components|StaticMesh|SetStaticMesh (Variables|/Game/Blueprints/Public/3DButton/BP_Char.BP_Char_C|GetStaticMesh _returnvalue) (Utilities|Array|Get(acopy) (Variables|Default|GetLetters) (Variables|Default|GetcurLetter)))
    (Rendering|Material|SetScalarParameterValueonMaterials (Variables|/Game/Blueprints/Public/3DButton/BP_Char.BP_Char_C|GetStaticMesh _returnvalue) "Color" (Utilities|Select :Index (Variables|Default|GetPalletteColor) :NewEnumerator0 0.01 :NewEnumerator1 0.1 :NewEnumerator2 0.2 :NewEnumerator3 0.3 :NewEnumerator4 0.4 :NewEnumerator10 0.5 :NewEnumerator5 0.6 :NewEnumerator6 0.7 :NewEnumerator9 1.0))
    (return _returnvalue)
    (else
      (return 0))))