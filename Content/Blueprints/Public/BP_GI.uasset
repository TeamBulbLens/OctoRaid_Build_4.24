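; Game instance for an asymmetric multiplayer game, routing the VR octopus and TPS players to their start maps by role.
; It creates, finds, joins and destroys sessions with status widget feedback, opens a listen-server lobby and server-travels between Lobby and Main.
; StartMainGame destroys the session before travel, and BackToLobby recreates it.
; It also allocates player UID slots, copied for Main, and serves a shuffleable skin list offset for an octopus host.
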(event Custom|ReadyForGame
  ;[1 1 1] 맵이동
  ;;[1 1 1] EntryMap에서 분기
  (bind _isoctopus (CallFunction|IsOctopus))
  (if _isoctopus
    (Game|OpenLevel(byName) "VRStart")
    (else
      (Game|OpenLevel(byName) "TPSStart"))))

(event Custom|Debug%20Show%20Collision
  ;[1 0.6443 0] Debug
  (if (Variables|Default|GetIsDebugMode)
    (Development|ExecuteConsoleCommand "Show Collision" 0)))

(event Custom|OpenLobby_Listen
  ;[1 1 1] 맵이동
  ;;[1 1 1] Lobby 리슨 서버로 열기
  (|Session (Game|GetPlayerController 0) (Variables|Default|GetMaxPlayerCount) false
    (:OnSuccess
      (Game|OpenLevel(byName) "Lobby" true "listen"))))

(event Custom|ConnectToListenServer
  (params (IP :type Name))
  (bind _returnvalue (Game|GetPlayerController 0))
  (bind _networksessionwidget (Variables|Default|GetNetworkSessionWidget))
  (bind _networksessionwidget_2 (Variables|Default|GetNetworkSessionWidget))
  (bind _networksessionwidget_3 (Variables|Default|GetNetworkSessionWidget))
  (bind _networksessionwidget_4 (Variables|Default|GetNetworkSessionWidget))
  ;[1 1 1] 맵이동
  ;;[1 1 1] 세션이 만들어졌는지 검색해서 연결
  (CallFunction|CreateNetworkWidget)
  (Utilities|IsValid _networksessionwidget
    (:Is%20Valid
      (Default|SetSearchSessionPanel _networksessionwidget "Visible")
      (bind _results (|FindSessions _returnvalue 5 false)
        (:OnSuccess
          (if (> (Utilities|Array|Length _results) 0)
            ;;[1 1 1] 게임 참가중 UI
            (Utilities|IsValid _networksessionwidget_4
              (:Is%20Valid
                (Default|SetSearchSessionPanel _networksessionwidget_4 "Collapsed")
                (Default|SetJoinSessionPanel _networksessionwidget_4 "Visible")
                (|JoinSession _returnvalue (Utilities|Array|Get(acopy) _results)
                  (:OnFailure
                    ;;[1 1 1] 게임참가 실패 UI
                    (Utilities|IsValid _networksessionwidget_3
                      (:Is%20Valid
                        (Default|SetJoinSessionPanel _networksessionwidget_3 "Collapsed")
                        (Default|SetFailedPanel _networksessionwidget_3 "Connection Failed. (Please try again.)")
                        (|DestroySession (Game|GetPlayerController 0))))))))
            (else
              ;;[1 1 1] 검색실패 UI
              (Utilities|IsValid _networksessionwidget_2 :!label _label
                (:Is%20Valid
                  (Default|SetSearchSessionPanel _networksessionwidget_2 "Collapsed")
                  (Default|SetFailedPanel _networksessionwidget_2 "Search Failed. (Lobby Generation check)"))))))
        (:OnFailure
          (goto _label))))))

(event Custom|BackToLobby
  ;[1 1 1] 맵이동
  (Utilities|FlowControl|Delay 1.0)
  (CallFunction|SetState "Ready")
  (|Session (Game|GetPlayerController 0) 5 false
    (:OnSuccess
      (CallFunction|ShowOctoLoading)
      (Development|ExecuteConsoleCommand "servertravel/Game/Maps/Lobby" 0))))

(event Custom|StartMainGame
  (params (DelayTime :type Float%20%28single-precision%29))
  ;[1 1 1] 맵이동
  (if (Utilities|Enum|Equal(Enum) (Variables|Default|GetCurrentState) "StartGame")
    _
    (else
      (|DestroySession (Game|GetPlayerController 0)
        (:OnSuccess
          (CallFunction|SetState "StartGame")))))
  (CallFunction|CopyHasUIDList)
  (Utilities|FlowControl|Delay DelayTime)
  (CallFunction|ShowOctoLoading)
  (Development|ExecuteConsoleCommand "servertravel/Game/Maps/Main" 0))

(event Custom|CreateNetworkWidget
  (bind _returnvalue (UserInterface|CreateWidget "/Game/Blueprints/Public/NetworkSessionWidget.NetworkSessionWidget_C" (Game|GetPlayerController 0)))
  (Variables|Default|SetNetworkSessionWidget _returnvalue)
  (UserInterface|Viewport|AddtoViewport (Variables|Default|GetNetworkSessionWidget) 0))

(event EventHandleNetworkError
  (params (FailureType :type ENetworkFailure%20Enum :default "NetDriverAlreadyExists") (bIsServer :type Boolean))
  (CallFunction|SetState "Ready")
  (|DestroySession (Game|GetPlayerController 0)))

(event EventInit
  ;[1 1 1] Init
  (CallFunction|SetHasUIDList)
  (CallFunction|SetState "Ready")
  (Skin|SetSkinList))

(fn SetGIRoleState
  (params (State :type ERoleState%20Enum :default "NewEnumerator0"))
  (Variables|Default|SetGI_RoleState State))

(fn IsOctopus
  (return (Utilities|Enum|Equal(Enum) (Variables|Default|GetGI_RoleState) "NewEnumerator0")))

(fn GetSkin
  (params (Index :type Integer))
  (bind _returnvalue (- Index 1))
  ;[1 1 1] 서버가 Octo일 때는 헌터플레이어 인덱스는 1부터 시작하니 빼준다
  (bind _isoctopus (CallFunction|IsOctopus))
  (if _isoctopus
    (if (>= _returnvalue 0)
      (return (Utilities|Array|Get(acopy) (Variables|Skin|GetSkins) _returnvalue)))
    (else
      (return (Utilities|Array|Get(acopy) (Variables|Skin|GetSkins) Index)))))

(fn SortSkinList
  (bind _skins (Variables|Skin|GetSkins))
  (bind _skins_2 (Variables|Skin|GetSkins))
  (bind _returnvalue (Utilities|Array|Length _skins_2))
  (for _index (range 0 (* (Utilities|Array|Length (Variables|Skin|GetSkins)) 3))
    (LocalVariables|SetIndex1 (Math|Random|RandomInteger _returnvalue))
    (LocalVariables|SetIndex2 (Math|Random|RandomInteger _returnvalue))
    (bind _output_get (LocalVariables|SetTemp (Utilities|Array|Get(acopy) _skins (LocalVariables|GetIndex1))))
    (Utilities|Array|SetArrayElem (Variables|Skin|GetSkins) (LocalVariables|GetIndex1) (Utilities|Array|Get(acopy) _skins (LocalVariables|GetIndex2)))
    (Utilities|Array|SetArrayElem (Variables|Skin|GetSkins) (LocalVariables|GetIndex2) _output_get)))

(fn SetSkinList
  (for _index (range 0 (- (|GetNumEnumEntries) 1))
    (Utilities|Array|Add (Variables|Skin|GetSkins) (Utilities|Enum|ByteToEnumESkinState (Math|Conversions|ToByte(Integer) _index)))))

(fn SetLocalUID
  (params (NewUID :type Integer))
  (Variables|Default|SetLocalUID NewUID))

(fn SetLocalSkinState
  (params (SkinState :type ESkinState%20Enum :default "NewEnumerator0"))
  (Variables|Skin|SetLocalSkinState SkinState))

(fn SetState
  (params (State :type EGameState%20Enum :default "Ready"))
  (Variables|Default|SetCurrentState State))

(fn SetHasUIDList
  (for _index (range 0 (- (Variables|Default|GetMaxPlayerCount) 1))
    (Utilities|Array|Add (Variables|Default|GetHasUIDList) false)))

(fn GetUID
  (bind _hasuidlist (Variables|Default|GetHasUIDList))
  (for (_array_element _array_index) _hasuidlist
    (if (not _array_element)
      (Utilities|Array|SetArrayElem _hasuidlist _array_index true)
      (return _array_index))))

(fn SetUIDEmpty
  (params (UID :type Integer))
  (Utilities|Array|SetArrayElem (Variables|Default|GetHasUIDList) UID false))

(fn CopyHasUIDList
  (Utilities|Array|Clear (Variables|Default|GetHasUIDList_Main))
  (for _array_element (Variables|Default|GetHasUIDList)
    (Utilities|Array|Add (Variables|Default|GetHasUIDList_Main) _array_element)))

(fn GetUIDMain
  (bind _hasuidlist_main (Variables|Default|GetHasUIDList_Main))
  (for (_array_element _array_index) _hasuidlist_main
    (if (not _array_element)
      (Utilities|Array|SetArrayElem _hasuidlist_main _array_index true)
      (return _array_index))))

(fn ShowOctoLoading
  (bind _asbp_vrpawn_main (Utilities|Casting|CastToBP_VRPawnMain (Game|Player|GetPlayerPawn 0)))
  (Default|SetLoadingMode _asbp_vrpawn_main))

(fn SetUIDMainEmpty
  (params (UID :type Integer))
  (Utilities|Array|SetArrayElem (Variables|Default|GetHasUIDList_Main) UID false))