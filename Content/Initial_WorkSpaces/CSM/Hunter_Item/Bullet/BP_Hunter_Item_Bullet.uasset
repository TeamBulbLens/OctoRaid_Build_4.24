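; BP_Hunter_Item_Bullet is an ammo pickup that raises MaxAmmo by 50 on the BP_PlayerCharacter_SN that overlaps it, then destroys itself.
; It spins in local space every tick at Rotatespeed, scaled by delta time.
; Its particle system activates after a short delay on BeginPlay.
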(event EventBeginPlay
  (Utilities|FlowControl|Delay 0.2)
  (Components|Activation|SetActive (Variables|Default|GetParticleSystem) true false))

(event Collision|EventActorBeginOverlap
  (params (OtherActor :type Actor%20Object%20Reference))
  (bind _asbp_player_character_sn (Utilities|Casting|CastToBP_PlayerCharacter_SN OtherActor))
  (Variables|/Game/Blueprints/SN/Blueprints_SN/BP_PlayerCharacter_SN.BP_PlayerCharacter_SN_C|SetMaxAmmo _asbp_player_character_sn (+ (Variables|/Game/Blueprints/SN/Blueprints_SN/BP_PlayerCharacter_SN.BP_PlayerCharacter_SN_C|GetMaxAmmo _asbp_player_character_sn) 50))
  (Actor|DestroyActor))

(event EventTick
  (params (DeltaSeconds :type Float%20%28single-precision%29))
  (Transformation|AddActorLocalRotation (* (Variables|Default|GetRotatespeed) (Utilities|Time|GetWorldDeltaSeconds)) false false))

(fn ConstructionScript)