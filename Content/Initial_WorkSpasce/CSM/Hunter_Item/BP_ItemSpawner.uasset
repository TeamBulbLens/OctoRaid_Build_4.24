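; BP_ItemSpawner respawns a hunter item at the spawner's transform after it leaves the spawner's sphere.
; Any end overlap sets IsSpawn and starts RespawnDelay, while a begin overlap by a BP_Hunter_Item-tagged actor clears it.
; If the flag survives the delay and the departing actor has that tag, ServerSpawnItem calls Respawn on authority, which spawns ItemToLoad and clears the flag.
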(event OnComponentBeginOverlap(Sphere)
  (params (OverlappedComponent :type Primitive%20Component%20Object%20Reference) (OtherActor :type Actor%20Object%20Reference) (OtherComp :type Primitive%20Component%20Object%20Reference) (OtherBodyIndex :type Integer) (bFromSweep :type Boolean) (SweepResult :type Hit%20Result%20Structure%20%28by%20ref%29))
  (if (Actor|ActorHasTag OtherActor "BP_Hunter_Item")
    (Variables|Default|SetIsSpawn? false)))

(event OnComponentEndOverlap(Sphere)
  (params (OverlappedComponent :type Primitive%20Component%20Object%20Reference) (OtherActor :type Actor%20Object%20Reference) (OtherComp :type Primitive%20Component%20Object%20Reference) (OtherBodyIndex :type Integer))
  (Variables|Default|SetIsSpawn? true)
  (Utilities|FlowControl|Delay (Variables|Default|GetRespawnDelay))
  (if (Variables|Default|GetIsSpawn?)
    (if (Actor|ActorHasTag OtherActor "BP_Hunter_Item")
      (CallFunction|ServerspawnItem))))

(event Custom|ServerSpawnItem
  (Networking|SwitchHasAuthority
    (:Authority
      (CallFunction|Respawn))))

(fn ConstructionScript)

(fn Respawn
  (if (Variables|Default|GetIsSpawn?)
    (Game|SpawnActorfromClass (Variables|Default|GetItemToLoad) (Transformation|GetActorTransform (Components|GetOwner (Variables|Default|GetItem_1))) "Undefined" 0 0)
    (Variables|Default|SetIsSpawn? false)
    (else
      (Variables|Default|SetIsSpawn? true))))