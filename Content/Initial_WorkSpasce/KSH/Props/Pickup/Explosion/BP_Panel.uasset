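; BP_Panel is an explosive two-sided screen pickup prop that breaks apart after being dropped.
; A hard hit or any box overlap, ignoring motion controllers, triggers destruction and explosion damage where a GameMode exists, effectively server-side.
; Destruction hides the mesh, spawns particles, relays sound through server and multicast events, then destroys the actor after a delay.
; The construction script builds front and back dynamic materials from per-side texture, color, panning and tiling variables.
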(event OnComponentBeginOverlap(Box)
  (params (OverlappedComponent :type Primitive%20Component%20Object%20Reference) (OtherActor :type Actor%20Object%20Reference) (OtherComp :type Primitive%20Component%20Object%20Reference) (OtherBodyIndex :type Integer) (bFromSweep :type Boolean) (SweepResult :type Hit%20Result%20Structure%20%28by%20ref%29))
  ;[1 1 1] 일정 이상의 충격이 가해지면 부서짐
  (if (Variables|Default|GetIsDropped)
    (Utilities|Casting|CastToBP_MotionControllerMain OtherActor
      (:CastFailed
        (Utilities|IsValid (Game|GetGameMode)
          (:Is%20Valid
            (CallFunction|Destruction)
            (CallFunction|ExplosionDamage)))))))

(event OnComponentHit(Box)
  (params (HitComponent :type Primitive%20Component%20Object%20Reference) (OtherActor :type Actor%20Object%20Reference) (OtherComp :type Primitive%20Component%20Object%20Reference) (NormalImpulse :type Vector :default "0, 0, 0") (Hit :type Hit%20Result%20Structure%20%28by%20ref%29))
  ;[1 1 1] 일정 이상의 충격이 가해지면 부서짐
  (if (Variables|Default|GetIsDropped)
    (Utilities|Casting|CastToBP_MotionControllerMain OtherActor
      (:CastFailed
        (Utilities|IsValid (Game|GetGameMode)
          (:Is%20Valid
            (if (> (Math|Vector|VectorLength NormalImpulse) 7e+05)
              (CallFunction|Destruction)
              (CallFunction|ExplosionDamage))))))))

(event Custom|CustomEvent
  (bind _returnvalue (Transformation|GetActorTransform))
  ;[1 1 1] 부서짐 효과
  (Physics|SetSimulatePhysics (Variables|Default|GetBox) false)
  (Collision|SetCollisionEnabled (Variables|Default|GetBox) "NoCollision")
  (Rendering|SetVisibility (Variables|Default|GetStaticMesh) false false)
  (Effects|SpawnEmitteratLocation (Variables|Default|GetExplosionEffect) (.location _returnvalue) (.rotation _returnvalue) (Variables|Default|GetScale))
  (CallFunction|PlaySound)
  (Utilities|FlowControl|Delay 2.0)
  (Actor|DestroyActor))

(event Custom|CustomEvent_1
  (params (SoundLocation :type Vector))
  ;[1 1 1] 폭발음
  (Audio|SpawnSoundatLocation "/Game/Ultimate_SFX_Bundle/Warfare_SFX_Bundle/Explosion_Sounds_Pro/Cues/Explosion.Explosion" SoundLocation "0, 0, 0" 1.0 1.0 0.0 0 0))

(event Custom|CustomEvent_2
  (params (SoundLocation :type Vector))
  ;[1 1 1] 폭발음
  (CallFunction|MulticastSound SoundLocation))

(event Custom|CustomEvent_3
  ;[1 1 1] 폭발음
  (CallFunction|ServerSound (.location (Transformation|GetActorTransform))))

(event Collision|EventActorBeginOverlap
  (params (OtherActor :type Actor%20Object%20Reference)))

(event EventTick
  (params (DeltaSeconds :type Float%20%28single-precision%29))
  (|CallParentFunction DeltaSeconds) ; 지금 이 노드는 비활성 상태입니다. \n핀을 끌어서 다른 노드를 연결하면 활성화됩니다.
)

(event EventBeginPlay
  (|CallParentFunction)
  (bind _asbp_gi (Utilities|Casting|CastToBP_GI (Game|GetGameInstance)))
  (if (Variables|/Game/Blueprints/Public/BP_GI.BP_GI_C|GetIsDebugMode _asbp_gi)
    _))

(fn ConstructionScript
  (bind _returnvalue (Rendering|Material|CreateDynamicMaterialInstance (Variables|Default|GetSM_Screen_Front) 0 "/Game/Neon_Materials/Materials/M_Panel/M_Panel.M_Panel" "MI_Screen_Front" :!class /Script/Engine.PrimitiveComponent))
  (Variables|Default|SetMI_Screen_Front _returnvalue)
  (bind _returnvalue_2 (Rendering|Material|CreateDynamicMaterialInstance (Variables|Default|GetSM_Screen_Back) 0 "/Game/Neon_Materials/Materials/M_Panel/M_Panel.M_Panel" "MI_Screen_Back" :!class /Script/Engine.PrimitiveComponent))
  (Variables|Default|SetMI_Screen_Back _returnvalue_2)
  (Utilities|FlowControl|Sequence
    (:then_0
      ;[1 1 1 1 28] Front Textures
      (Rendering|Material|SetTextureParameterValue (Variables|Default|GetMI_Screen_Front) "Opacity Map" (Variables|TexturesFront|GetOpacity%20Map%20Front))
      (Rendering|Material|SetTextureParameterValue (Variables|Default|GetMI_Screen_Front) "Base Color Map" (Variables|TexturesFront|GetBase%20Color%20Front))
      (Rendering|Material|SetTextureParameterValue (Variables|Default|GetMI_Screen_Front) "Pixel Map" (Variables|TexturesFront|GetPixel%20Map%20Front))
      ;[1 1 1 1 28] Back Textures
      (Rendering|Material|SetTextureParameterValue (Variables|Default|GetMI_Screen_Back) "Opacity Map" (Variables|TexturesBack|GetOpacity%20Map%20Back))
      (Rendering|Material|SetTextureParameterValue (Variables|Default|GetMI_Screen_Back) "Base Color Map" (Variables|TexturesBack|GetBase%20Color%20Back))
      (Rendering|Material|SetTextureParameterValue (Variables|Default|GetMI_Screen_Back) "Pixel Map" (Variables|TexturesBack|GetPixel%20Map%20Back)))
    (:then_1
      ;[1 1 1 1 28] Front Color and Emissive
      (Rendering|Material|SetVectorParameterValue (Variables|Default|GetMI_Screen_Front) "Background Color" (Variables|ColorFront|GetBackground%20Color%20Front) :!class /Script/Engine.MaterialInstanceDynamic)
      (Rendering|Material|SetScalarParameterValue (Variables|Default|GetMI_Screen_Front) "Emissive" (Variables|ColorFront|GetEmissive%20Front) :!class /Script/Engine.MaterialInstanceDynamic)
      (Rendering|Material|SetScalarParameterValue (Variables|Default|GetMI_Screen_Front) "Desaturation" (Variables|ColorFront|GetDesaturation%20Front) :!class /Script/Engine.MaterialInstanceDynamic)
      (Rendering|Material|SetScalarParameterValue (Variables|Default|GetMI_Screen_Front) "Hue" (Variables|ColorFront|GetHue%20Front) :!class /Script/Engine.MaterialInstanceDynamic)
      ;[1 1 1 1 28] Back Color and Emissive
      (Rendering|Material|SetVectorParameterValue (Variables|Default|GetMI_Screen_Back) "Background Color" (Variables|ColorBack|GetBackground%20Color%20Back) :!class /Script/Engine.MaterialInstanceDynamic)
      (Rendering|Material|SetScalarParameterValue (Variables|Default|GetMI_Screen_Back) "Emissive" (Variables|ColorBack|GetEmissive%20Back) :!class /Script/Engine.MaterialInstanceDynamic)
      (Rendering|Material|SetScalarParameterValue (Variables|Default|GetMI_Screen_Back) "Desaturation" (Variables|ColorBack|GetDesaturation%20Back) :!class /Script/Engine.MaterialInstanceDynamic)
      (Rendering|Material|SetScalarParameterValue (Variables|Default|GetMI_Screen_Back) "Hue" (Variables|ColorBack|GetHue%20Back) :!class /Script/Engine.MaterialInstanceDynamic))
    (:then_2
      ;[1 1 1 1 28] Front Panners
      (Rendering|Material|SetScalarParameterValue (Variables|Default|GetMI_Screen_Front) "X Panner" (Variables|PannerFront|GetX_Panner%20Front) :!class /Script/Engine.MaterialInstanceDynamic)
      (Rendering|Material|SetScalarParameterValue (Variables|Default|GetMI_Screen_Front) "Y Panner" (Variables|PannerFront|GetY_Panner%20Front) :!class /Script/Engine.MaterialInstanceDynamic)
      ;[1 1 1 1 28] Back Panners
      (Rendering|Material|SetScalarParameterValue (Variables|Default|GetMI_Screen_Back) "X Panner" (Variables|PannerBack|GetX_Panner%20Back) :!class /Script/Engine.MaterialInstanceDynamic)
      (Rendering|Material|SetScalarParameterValue (Variables|Default|GetMI_Screen_Back) "Y Panner" (Variables|PannerBack|GetY_Panner%20Back) :!class /Script/Engine.MaterialInstanceDynamic))
    (:then_3
      ;[1 1 1 1 28] Front UV Tiling
      (Rendering|Material|SetScalarParameterValue (Variables|Default|GetMI_Screen_Front) "U Tiling" (Variables|TilingFront|GetU%20Tiling%20Front) :!class /Script/Engine.MaterialInstanceDynamic)
      (Rendering|Material|SetScalarParameterValue (Variables|Default|GetMI_Screen_Front) "V Tiling" (Variables|TilingFront|GetV%20Tiling%20Front) :!class /Script/Engine.MaterialInstanceDynamic)
      ;[1 1 1] Comment
      (Rendering|Material|SetScalarParameterValue (Variables|Default|GetMI_Screen_Back) "U Tiling" (Variables|TilingBack|GetU%20Tiling%20Back) :!class /Script/Engine.MaterialInstanceDynamic)
      (Rendering|Material|SetScalarParameterValue (Variables|Default|GetMI_Screen_Back) "V Tiling" (Variables|TilingBack|GetV%20Tiling%20Back) :!class /Script/Engine.MaterialInstanceDynamic))))