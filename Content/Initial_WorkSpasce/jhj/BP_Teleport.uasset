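; BP_Teleport is a sewer teleporter actor that warps the player pawn to the location of its component A after a delay.
; A Box overlap hides the Sewer component, shows the Portal and starts a five-second wait.
; If the overlap flag is still set and the overlapping actor has the "Octo" tag, player pawn 0 teleports with zero rotation.
; Ending the actor overlap clears the flag and restores the Sewer visual.
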(event OnComponentBeginOverlap(Box)
  (params (OverlappedComponent :type Primitive%20Component%20Object%20Reference) (OtherActor :type Actor%20Object%20Reference) (OtherComp :type Primitive%20Component%20Object%20Reference) (OtherBodyIndex :type Integer) (bFromSweep :type Boolean) (SweepResult :type Hit%20Result%20Structure%20%28by%20ref%29))
  ;[1 1 1] 워프
  (Rendering|SetVisibility (Variables|Default|GetSewer) false false)
  (Rendering|SetVisibility (Variables|Default|GetPortal) true false)
  (Variables|Default|Setisoverlap true)
  (Utilities|FlowControl|Delay 5.0)
  (if (Variables|Default|Getisoverlap)
    (if (Actor|ActorHasTag OtherActor "Octo")
      (Transformation|Teleport (Game|Player|GetPlayerPawn 0) (Transformation|GetWorldLocation (Variables|Default|GetA)) "0, 0, 0")
      (Rendering|SetVisibility (Variables|Default|GetSewer) true false)
      (Rendering|SetVisibility (Variables|Default|GetPortal) false false))))

(event EventBeginPlay)

(event Collision|EventActorBeginOverlap
  (params (OtherActor :type Actor%20Object%20Reference)))

(event EventTick
  (params (DeltaSeconds :type Float%20%28single-precision%29)))

(event Collision|EventActorEndOverlap
  (params (OtherActor :type Actor%20Object%20Reference))
  ;[1 1 1] 워프
  (Variables|Default|Setisoverlap false)
  (Rendering|SetVisibility (Variables|Default|GetSewer) true false)
  (Rendering|SetVisibility (Variables|Default|GetPortal) false false))

(fn ConstructionScript)